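; BPC_ComponenteSalud is a health component that tracks an actor's current and maximum life.
; DisminuirVida subtracts damage, clamps the result between zero and the maximum, and sets the EstaMuerto death flag.
; It then broadcasts the new values through the ActualizarVida dispatcher and prints debug messages for health and death.
; The event graph holds only disabled placeholder events, and SeMamut is an empty stub.
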(event EventBeginPlay)

(event EventTick
  (params (DeltaSeconds :type Float%20%28single-precision%29)))

(fn DisminuirVida
  (params (Daño :type Float%20%28double-precision%29))
  (bind _output_get (Variables|Default|SetVidaActual (Math|Float|Clamp(Float) (- (Variables|Default|GetVidaActual) Daño) 0.0 (Variables|Default|GetVidaMaxima))))
  (Variables|Default|SetbEstaMuerto? (<= _output_get 0.0))
  (Default|CallActualizarVida (Variables|Default|GetVidaActual) (Variables|Default|GetVidaMaxima))
  (Development|PrintString (Utilities|String|Append "La vida actual es" (Utilities|String|ToString(Float) (Variables|Default|GetVidaActual))))
  (if (Variables|Default|GetbEstaMuerto?)
    (Development|PrintString "Se murio")))

(fn SeMamut)